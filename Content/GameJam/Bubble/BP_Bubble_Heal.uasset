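; BP_Bubble_Heal is a healing bubble pickup that restores a player's bubble value on contact.
; When its collision sphere is overlapped, it ignores the contact during a very brief window after spawn, gated by Lifetime.
; Otherwise, if the other actor is a BP_Player_Base, it passes its Quality to ChangeBubbleVal and destroys itself.
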(event OnComponentBeginOverlap(SphereCollision)
  (params (OverlappedComponent :type Primitive%20Component%20Object%20Reference) (OtherActor :type Actor%20Object%20Reference) (OtherComp :type Primitive%20Component%20Object%20Reference) (OtherBodyIndex :type Integer) (bFromSweep :type Boolean) (SweepResult :type Hit%20Result%20Structure%20%28by%20ref%29))
  (if (not (< (Variables|Default|GetLifetime) 0.02))
    (bind _asbp_player_base (Utilities|Casting|CastToBP_Player_Base OtherActor))
    ;[1 1 1] 恢复人物泡泡
    (if (Utilities|IsValid _asbp_player_base)
      (Default|ChangeBubbleVal _asbp_player_base (Variables|Default|GetQuality))
      (Actor|DestroyActor))))

(event EventBeginPlay
  (|CallParentFunction) ; 此节点被禁用，将不会被调用。\n从引脚连出引线来编译功能。
)

(event Collision|EventActorBeginOverlap
  (params (OtherActor :type Actor%20Object%20Reference))
  (|CallParentFunction OtherActor) ; 此节点被禁用，将不会被调用。\n从引脚连出引线来编译功能。
)

(event EventTick
  (params (DeltaSeconds :type Float%20%28single-precision%29))
  (|CallParentFunction DeltaSeconds) ; 此节点被禁用，将不会被调用。\n从引脚连出引线来编译功能。
)

(fn ConstructionScript
  (|CallParentFunction))