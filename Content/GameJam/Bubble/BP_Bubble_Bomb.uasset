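; BP_Bubble_Bomb is a bubble projectile that explodes on overlap after a brief spawn grace period.
; Touching BP_Poisonous instead replaces it with a BP_Bubble_Poisonous that receives its ProjectileMovement reference.
; Otherwise, class-filtered players inside BombRange are launched outward, scaled by their IncreaseDamage, and receive health and random IncreaseDamage changes before the bomb destroys itself.
; The physics-force fallback sits behind the player cast, and the deceleration logic is unconnected.
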(event OnComponentBeginOverlap(SphereCollision)
  (params (OverlappedComponent :type Primitive%20Component%20Object%20Reference) (OtherActor :type Actor%20Object%20Reference) (OtherComp :type Primitive%20Component%20Object%20Reference) (OtherBodyIndex :type Integer) (bFromSweep :type Boolean) (SweepResult :type Hit%20Result%20Structure%20%28by%20ref%29))
  (bind _forceval (Variables|Default|GetForceVal))
  (if (not (< (Variables|Default|GetLifetime) 0.02))
    (Utilities|Casting|CastToBP_Poisonous OtherActor
      (:then
        (bind _returnvalue (Game|SpawnActorfromClass "/Game/GameJam/Bubble/BP_Bubble_Poisonous.BP_Bubble_Poisonous_C" (Transformation|GetActorTransform self) "Undefined" "MultiplyWithRoot" 0 0))
        (Variables|/Game/GameJam/Bubble/BP_Bubble_Base.BP_Bubble_Base_C|SetProjectileMovement _returnvalue (Variables|Default|GetProjectileMovement))
        (Actor|DestroyActor))
      (:CastFailed
        (for _array_element (Variables|Default|GetClass%20Filter)
          (for _array_element_2 (Collision|GetOverlappingActors (Variables|组件|GetBombRange) _array_element :!class /Script/Engine.PrimitiveComponent)
            (bind _asbp_player_base (Utilities|Casting|CastToBP_Player_Base _array_element_2))
            ;[1 1 1] 获取Character,扣血，和增伤
            (if (Utilities|IsValid _asbp_player_base)
              (Character|LaunchCharacter _asbp_player_base (* (* (Math|Vector|Normalize (- (Transformation|GetActorLocation _array_element_2) (Transformation|GetActorLocation self))) (Math|Vector|MakeVector _forceval _forceval _forceval)) (Math|Vector|MakeVector (+ (* (/ (Variables|/Game/GameJam/Character/BP_Player_Base.BP_Player_Base_C|GetIncreaseDamage _asbp_player_base) 1e+02) 2e+01) 1e+01) (+ (* (/ (Variables|/Game/GameJam/Character/BP_Player_Base.BP_Player_Base_C|GetIncreaseDamage _asbp_player_base) 1e+02) 2e+01) 1e+01) (+ (* (/ (Variables|/Game/GameJam/Character/BP_Player_Base.BP_Player_Base_C|GetIncreaseDamage _asbp_player_base) 1e+02) 2e+01) 1e+01))) false false)
              (Default|ChangeHealth _asbp_player_base (Variables|Default|GetDamageVal))
              (Default|ChangeIncreaseDamage _asbp_player_base (Math|Random|RandomFloatinRange (Math|Float|MakeLiteralFloat 2.0) (Variables|Default|GetBubbleIncreaseDamage)))
              (else
                (Physics|AddForce (Actor|GetComponentbyClass _array_element_2 "/Script/Engine.PrimitiveComponent") (* (Math|Vector|Normalize (- (Transformation|GetActorLocation _array_element_2) (Transformation|GetActorLocation self))) (Math|Vector|MakeVector _forceval _forceval _forceval)) "None" false)))))
        (Actor|DestroyActor)))))

(event Collision|EventActorBeginOverlap
  (params (OtherActor :type Actor%20Object%20Reference)))

(fn ConstructionScript)

(fn 新函数)