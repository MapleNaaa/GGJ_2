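; Poisonous bubble pickup or hazard that costs players health and changes their damage-increase value on contact, then destroys itself.
; When its collision sphere begins an overlap, it loops through all overlapping BP_Player_Base actors.
; Each valid player receives ChangeHealth with DamageVal and ChangeIncreaseDamage with BubbleIncreaseDamage, and DestroyActor is called inside the loop.
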(event OnComponentBeginOverlap(SphereCollision)
  (params (OverlappedComponent :type Primitive%20Component%20Object%20Reference) (OtherActor :type Actor%20Object%20Reference) (OtherComp :type Primitive%20Component%20Object%20Reference) (OtherBodyIndex :type Integer) (bFromSweep :type Boolean) (SweepResult :type Hit%20Result%20Structure%20%28by%20ref%29))
  (for _array_element (Collision|GetOverlappingActors (Variables|Default|GetSphereCollision) "/Game/GameJam/Character/BP_Player_Base.BP_Player_Base_C" :!class /Script/Engine.PrimitiveComponent)
    ;[1 1 1] 获取Character,扣血，和增伤
    (bind _asbp_player_base (Utilities|Casting|CastToBP_Player_Base _array_element))
    (if (Utilities|IsValid _asbp_player_base)
      (Default|ChangeHealth _asbp_player_base (Variables|Default|GetDamageVal))
      (Default|ChangeIncreaseDamage _asbp_player_base (Variables|Default|GetBubbleIncreaseDamage))
      (Actor|DestroyActor))))

(event EventBeginPlay)

(event Collision|EventActorBeginOverlap
  (params (OtherActor :type Actor%20Object%20Reference)))

(event EventTick
  (params (DeltaSeconds :type Float%20%28single-precision%29)))

(fn ConstructionScript)