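; Base player character for a bubble-combat game, holding health and a bubble value that lowers walk speed as it rises.
; Tick refreshes speed and both percentages, while movement input follows control yaw.
; Attack fires a hold-scaled bubble bomb that spends bubble value and, when lock is toggled on, faces another player; a held prop is used instead, then reverts to bombs.
; Dodge launches the character, and Spawn randomly sheds small bubbles.
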(event EventTick
  (params (DeltaSeconds :type Float%20%28single-precision%29))
  (Variables|/Script/Engine.CharacterMovementComponent|SetMaxWalkSpeed (Variables|Character|GetCharacterMovement) (* (- (Math|Float|MakeLiteralFloat 1.2e+02) (Variables|Default|GetBubbleVal)) 1e+02))
  (Variables|Default|SetHealthPercent (/ (Variables|Default|GetHealth) (Variables|Default|GetMaxHealth)))
  (Variables|Default|SetBubbleValPercent (/ (Variables|Default|GetBubbleVal) (Variables|Default|GetMaxBubbleVal)))
  (if (> (Math|Vector|VectorLength (Variables|/Script/Engine.MovementComponent|GetVelocity (Variables|Character|GetCharacterMovement))) 1e+02)
    _))

(event Input|EnhancedActionEvents|EnhancedInputActionP0_Movement
  (params (ActionValue :type Vector%202D%20Structure) (ElapsedSeconds :type Float%20%28double-precision%29) (TriggeredSeconds :type Float%20%28double-precision%29) (InputAction :type Input%20Action%20Object%20Reference :default "/Game/TopDown/Input/Actions/P0_Movement.P0_Movement"))
  (bind _returnvalue (Pawn|GetControlRotation :!class /Script/Engine.Pawn))
  (bind _returnvalue_2 (Math|Rotator|MakeRotator 0.0 0.0 (.yaw _returnvalue)))
  (Utilities|FlowControl|Sequence
    (:then_0
      (Pawn|Input|AddMovementInput (Math|Vector|GetForwardVector _returnvalue_2) (.x ActionValue) false))
    (:then_1
      (Pawn|Input|AddMovementInput (Math|Vector|GetRightVector _returnvalue_2) (.y ActionValue) false))))

(fn ConstructionScript)

(fn ChangeBubbleVal
  (params (ChangedVal :type Float%20%28double-precision%29))
  (Variables|Default|SetBubbleVal (+ ChangedVal (Variables|Default|GetBubbleVal))))

(fn ChangeHealth
  (params (ChangedVal :type Float%20%28double-precision%29))
  (Variables|Default|SetHealth (+ ChangedVal (Variables|Default|GetHealth))))

(fn ChangeIncreaseDamage
  (params (ChangedVal :type Float%20%28double-precision%29))
  (Variables|Default|SetIncreaseDamage (+ ChangedVal (Variables|Default|GetIncreaseDamage))))

(fn Attack
  (params (HoldTime :type Float%20%28double-precision%29))
  (bind _returnvalue (/ HoldTime 1.0))
  (bind _self self)
  (bind _self_2 self)
  (bind _returnvalue_2 (Transformation|GetActorTransform _self))
  (bind _returnvalue_3 (Math|Float|Min(Float) _returnvalue 3.0))
  (if (== (Variables|Default|GetSpawnedClass) "/Game/GameJam/Bubble/BP_Bubble_Bomb.BP_Bubble_Bomb_C")
    (bind _returnvalue_4 (Game|SpawnActorfromClass (Variables|Default|GetSpawnedClass) (Math|Transform|MakeTransform (+ (.location _returnvalue_2) (Math|Vector|RotateVector (Variables|Default|GetOffset) (.rotation _returnvalue_2))) (.rotation _returnvalue_2) (Math|Vector|MakeVector _returnvalue_3 _returnvalue_3 _returnvalue_3)) "Undefined" "MultiplyWithRoot" 0 0))
    (bind _asbp_bubble_base (Utilities|Casting|CastToBP_Bubble_Base _returnvalue_4))
    (if (Utilities|IsValid _asbp_bubble_base)
      (Variables|Default|SetBubbleVal (- (Variables|Default|GetBubbleVal) (* _returnvalue_3 (Variables|/Game/GameJam/Bubble/BP_Bubble_Base.BP_Bubble_Base_C|GetQuality _asbp_bubble_base))))
      (if (Variables|Default|GetIsLocking)
        (bind _outactors (Actor|GetAllActorsOfClass "BP_Player_Base_C"))
        (for _array_element _outactors
          (if (!= _array_element _self_2)
            (Transformation|SetActorRotation _asbp_bubble_base (Class|KismetMathLibrary|QuatRotator (Math|Conversions|ToQuaternion(Rotator) (- (Transformation|GetActorLocation _array_element) (Transformation|GetActorLocation _self_2)))))))))
    (else
      (Variables|Default|SetIsUsed false)
      (bind _returnvalue_5 (Game|SpawnActorfromClass (Variables|Default|GetSpawnedClass) (Math|Transform|MakeTransform (- (.location _returnvalue_2) "0.000000,0.000000,-100.000000") (.rotation _returnvalue_2) (.scale _returnvalue_2)) "Undefined" "MultiplyWithRoot" 0 0))
      (bind _asbp_prop_base (Utilities|Casting|CastToBP_Prop_Base _returnvalue_5))
      (if (Utilities|IsValid _asbp_prop_base)
        (Default|UseProp _asbp_prop_base)
        (Variables|Default|SetSpawnedClass "/Game/GameJam/Bubble/BP_Bubble_Bomb.BP_Bubble_Bomb_C")))))

(fn Dodge
  (Variables|Default|SetIsDodge true)
  (Character|LaunchCharacter (Math|Vector|RotateVector (Variables|Default|GetLaunchDistance) (.rotation (Transformation|GetActorTransform self))) false false))

(fn Spawn
  (bind _self self)
  (bind _returnvalue (Transformation|GetActorTransform _self))
  (if (< (Math|Random|RandomIntegerinRange 10 0) 5)
    (bind _output_get (LocalVariables|SetNewLocalVar (* (Math|Conversions|ToFloat(Integer) (Math|Random|RandomIntegerinRange 3 1)) 0.2)))
    (Variables|Default|SetBubbleVal (- (Variables|Default|GetBubbleVal) _output_get))
    (Game|SpawnActorfromClass "/Game/GameJam/Bubble/BP_Bubble_Base.BP_Bubble_Base_C" (Math|Transform|MakeTransform (+ (.location _returnvalue) (Math|Vector|RotateVector (Variables|Default|GetOffset) (.rotation _returnvalue))) (.rotation _returnvalue) (Math|Vector|MakeVector _output_get _output_get _output_get)) "Undefined" "MultiplyWithRoot" 0 0)))

(fn Lock
  (Utilities|FlowControl|FlipFlop
    (:A
      (Variables|Default|SetIsLocking true))
    (:B
      (Variables|Default|SetIsLocking false))))