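; BP_Player02 is the second player's character Blueprint for a game jam project with a shared controller.
; When possessed with a player controller index above zero, it finds the first BP_SharedController in the level and stores itself as that controller's Player02.
; The other event stubs are disabled, and the construction script only calls the parent.
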(event EventBeginPlay)

(event Collision|EventActorBeginOverlap
  (params (OtherActor :type Actor%20Object%20Reference)))

(event EventTick
  (params (DeltaSeconds :type Float%20%28single-precision%29))
  (|CallParentFunction DeltaSeconds) ; 此节点被禁用，将不会被调用。\n从引脚连出引线来编译功能。
)

(event EventPossessed
  (params (NewController :type Controller%20Object%20Reference))
  (if (> (Variables|Default|GetPlayerControllerIndex) 0)
    (bind _outactors (Actor|GetAllActorsOfClass "/Game/GameJam/Character/BP_SharedController.BP_SharedController_C"))
    (Variables|/Game/GameJam/Character/BP_SharedController.BP_SharedController_C|SetPlayer02 (Utilities|Array|Get(acopy) _outactors) self)))

(fn ConstructionScript
  (|CallParentFunction))