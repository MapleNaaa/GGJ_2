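; BP_Prop_XieYao is a laxative prop pickup that grants players a poisonous bubble.
; When a player overlaps its sphere, it sets that player's spawn class to BP_Bubble_Poisonous, clears the used flag and destroys itself.
; UseProp records the owner's transform after calling the parent.
; A separate SpawnPoisonous event, with no caller here, waits briefly, then spawns a scaled, damage-multiplied bubble at that saved transform.
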(event OnComponentBeginOverlap(Sphere)
  (params (OverlappedComponent :type Primitive%20Component%20Object%20Reference) (OtherActor :type Actor%20Object%20Reference) (OtherComp :type Primitive%20Component%20Object%20Reference) (OtherBodyIndex :type Integer) (bFromSweep :type Boolean) (SweepResult :type Hit%20Result%20Structure%20%28by%20ref%29))
  (bind _output_get (Variables|Default|SetTheOwner OtherActor))
  (bind _asbp_player_base (Utilities|Casting|CastToBP_Player_Base _output_get))
  (Variables|/Game/GameJam/Character/BP_Player_Base.BP_Player_Base_C|SetSpawnedClass _asbp_player_base "/Game/GameJam/Bubble/BP_Bubble_Poisonous.BP_Bubble_Poisonous_C")
  (Variables|/Game/GameJam/Character/BP_Player_Base.BP_Player_Base_C|SetIsUsed _asbp_player_base false)
  (Actor|DestroyActor))

(event Custom|SpawnPoisonous
  (bind _scaleval (Variables|Default|GetScaleVal))
  (Utilities|FlowControl|Delay 2.0)
  (bind _returnvalue (Game|SpawnActorfromClass "/Game/GameJam/Bubble/BP_Bubble_Poisonous.BP_Bubble_Poisonous_C" (Variables|Default|GetBeforeTransform) "Undefined" "MultiplyWithRoot" 0 0))
  (Variables|/Game/GameJam/Bubble/BP_Bubble_Base.BP_Bubble_Base_C|SetDamageVal _returnvalue (* (Variables|/Game/GameJam/Bubble/BP_Bubble_Base.BP_Bubble_Base_C|GetDamageVal _returnvalue) (Variables|Default|GetDamageUpTimes)))
  (Transformation|SetActorScale3D _returnvalue (Math|Vector|MakeVector _scaleval _scaleval _scaleval)))

(event EventBeginPlay
  (|CallParentFunction) ; 此节点被禁用，将不会被调用。\n从引脚连出引线来编译功能。
)

(event Collision|EventActorBeginOverlap
  (params (OtherActor :type Actor%20Object%20Reference))
  (|CallParentFunction OtherActor) ; 此节点被禁用，将不会被调用。\n从引脚连出引线来编译功能。
)

(event EventTick
  (params (DeltaSeconds :type Float%20%28single-precision%29))
  (|CallParentFunction DeltaSeconds) ; 此节点被禁用，将不会被调用。\n从引脚连出引线来编译功能。
)

(fn ConstructionScript
  (|CallParentFunction))

(fn UseProp
  (|CallParentFunction)
  (Variables|Default|SetBeforeTransform (Transformation|GetActorTransform (Variables|Default|GetTheOwner))))