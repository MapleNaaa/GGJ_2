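; Spawner actor that drops a BP_Prop_XieYao prop between the two players.
; Tick accumulates LifeTime and passes when its whole-second value is a multiple of twenty, guarded by an IsSpawn flag.
; The prop spawns at the midpoint of player 0 and 1 pawns, lowered slightly in Z.
; IsSpawn is never reset here, so the spawn happens only once despite the periodic check.
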(event EventBeginPlay)

(event Collision|EventActorBeginOverlap
  (params (OtherActor :type Actor%20Object%20Reference)))

(event EventTick
  (params (DeltaSeconds :type Float%20%28single-precision%29))
  (bind _returnvalue (Game|GetPlayerController 1))
  (bind _returnvalue_2 (Pawn|GetControlledPawn _returnvalue))
  (bind _returnvalue_3 (Transformation|GetActorLocation _returnvalue_2))
  (Variables|Default|SetLifeTime (+ DeltaSeconds (Variables|Default|GetLifeTime)))
  (if (== (Class|KismetMathLibrary|PercentInt64Int64 (Class|KismetMathLibrary|ToInt64(Float) (Variables|Default|GetLifeTime)) 20) 0)
    (if (not (Variables|Default|GetIsSpawn))
      (Variables|Default|SetIsSpawn true)
      (Game|SpawnActorfromClass "/Game/GameJam/Props/BP_Prop_XieYao.BP_Prop_XieYao_C" (Math|Transform|MakeTransform (- (+ (/ (- (Transformation|GetActorLocation (Pawn|GetControlledPawn (Game|GetPlayerController 0))) _returnvalue_3) "2.000000,2.000000,2.000000") _returnvalue_3) "0.000000,0.000000,100.000000") "0, 0, 0" "1.000000,1.000000,1.000000") "Undefined" "MultiplyWithRoot" 0 0))))

(fn ConstructionScript)