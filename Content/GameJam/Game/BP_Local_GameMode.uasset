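; Game mode for a two-player local multiplayer match that spawns and possesses both players' pawns.
; On BeginPlay it gathers the level's PlayerStarts and spawns BP_Player01 and BP_Player02 at the first two.
; Player one is possessed by the existing controller, while player two gets one from CreatePlayer.
; Each pawn receives its controller index and its own tag.
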(event EventBeginPlay
  (bind _returnvalue (Game|GetPlayerController 0))
  (bind _outactors (Actor|GetAllActorsOfClass "/Script/Engine.PlayerStart"))
  (for _index (range 0 1)
    (if (> _index 0)
      (bind _returnvalue_2 (Class|GameplayStatics|CreatePlayer -1))
      (bind _returnvalue_3 (Game|SpawnActorfromClass "/Game/GameJam/Character/BP_Player02.BP_Player02_C" (Transformation|GetActorTransform (Utilities|Array|Get(acopy) _outactors _index)) "Undefined" "MultiplyWithRoot" 0 0))
      (Variables|/Game/GameJam/Character/BP_Player_Base.BP_Player_Base_C|SetPlayerControllerIndex _returnvalue_3 _index)
      (Pawn|Possess _returnvalue_2 _returnvalue_3)
      (Variables|/Script/Engine.Actor|SetTags _returnvalue_3 (Variables|Default|GetTag02))
      (else
        (bind _returnvalue_4 (Game|SpawnActorfromClass "/Game/GameJam/Character/BP_Player01.BP_Player01_C" (Transformation|GetActorTransform (Utilities|Array|Get(acopy) _outactors _index)) "Undefined" "MultiplyWithRoot" _returnvalue 0))
        (Variables|/Game/GameJam/Character/BP_Player_Base.BP_Player_Base_C|SetPlayerControllerIndex _returnvalue_4 0)
        (Pawn|Possess _returnvalue _returnvalue_4)
        (Variables|/Script/Engine.Actor|SetTags _returnvalue_4 (Variables|Default|GetTag01))))))

(event EventTick
  (params (DeltaSeconds :type Float%20%28single-precision%29)))

(fn ConstructionScript)