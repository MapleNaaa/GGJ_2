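; BP_Outermost is a hazard volume, likely for the outer edge of the level, intended to instantly kill players who stay inside it.
; When a BP_Player_Base begins overlapping its BoxCollision, it waits briefly, then re-queries the box's overlapping players.
; Each player still inside receives a large negative ChangeHealth, so anyone who leaves during the delay is spared by that check.
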(event OnComponentBeginOverlap(BoxCollision)
  (params (OverlappedComponent :type Primitive%20Component%20Object%20Reference) (OtherActor :type Actor%20Object%20Reference) (OtherComp :type Primitive%20Component%20Object%20Reference) (OtherBodyIndex :type Integer) (bFromSweep :type Boolean) (SweepResult :type Hit%20Result%20Structure%20%28by%20ref%29))
  (bind _asbp_player_base (Utilities|Casting|CastToBP_Player_Base OtherActor))
  (if (Utilities|IsValid _asbp_player_base)
    (Utilities|FlowControl|Delay 0.5)
    ;[1 1 1] 秒杀
    (for _array_element (Collision|GetOverlappingActors (Variables|Default|GetBoxCollision) "/Game/GameJam/Character/BP_Player_Base.BP_Player_Base_C" :!class /Script/Engine.PrimitiveComponent)
      (bind _asbp_player_base_2 (Utilities|Casting|CastToBP_Player_Base _array_element))
      (if (Utilities|IsValid _asbp_player_base_2)
        (Default|ChangeHealth _asbp_player_base_2 -1e+02)))))

(event EventBeginPlay)

(event Collision|EventActorBeginOverlap
  (params (OtherActor :type Actor%20Object%20Reference)))

(event EventTick
  (params (DeltaSeconds :type Float%20%28single-precision%29)))

(fn ConstructionScript)